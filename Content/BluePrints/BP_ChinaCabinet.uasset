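; BP_ChinaCabinet is a noise hazard that makes a crash sound when the player bumps into it and alerts nearby parent listeners.
; A Box overlap by BP_Player plays CabinetCrash at the Cabinet component's location.
; It then queries the NoiseRange component for overlapping BP_ParentListener actors and calls AddNoise on each.
; The sound and noise fire on every new overlap, with no cooldown or one-shot guard.
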(event OnComponentBeginOverlap(Box)
  (params (OverlappedComponent :type Primitive%20Component%20Object%20Reference) (OtherActor :type Actor%20Object%20Reference) (OtherComp :type Primitive%20Component%20Object%20Reference) (OtherBodyIndex :type Integer) (bFromSweep :type Boolean) (SweepResult :type Hit%20Result%20Structure%20%28by%20ref%29))
  (bind _noiserange (Variables|Default|GetNoiseRange))
  (Utilities|Casting|CastToBP_Player OtherActor)
  (Audio|PlaySoundatLocation "/Game/Sounds/CabinetCrash.CabinetCrash" (Transformation|GetWorldLocation (Variables|Default|Get%20Cabinet)) "0, 0, 0" 1.0 1.0 0.0 0 0 0 0)
  (bind _outactors (Collision|ComponentOverlapActors _noiserange (Transformation|GetWorldTransform _noiserange) (Utilities|Array|MakeArray "ObjectTypeQuery2") "/Game/BluePrints/BP_ParentListener.BP_ParentListener_C"))
  (for _array_element _outactors
    (bind _asbp_parent_listener (Utilities|Casting|CastToBP_ParentListener _array_element))
    (Default|AddNoise _asbp_parent_listener)))

(event EventBeginPlay)

(event Collision|EventActorBeginOverlap
  (params (OtherActor :type Actor%20Object%20Reference)))

(event EventTick
  (params (DeltaSeconds :type Float%20%28single-precision%29)))

(fn ConstructionScript)