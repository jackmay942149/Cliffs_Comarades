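; Player character for directional melee combat, with Enhanced Input movement, attacking, blocking and chest opening.
; Shifting sides mirrors the mesh by negative X scale; attack and block montages cut look sensitivity, which Tick eases back.
; HitDetection traces from the hand to notify enemies, while incoming hits only print Blocked or Hit from block state and side offsets.
; Opening a traced chest shows a random spoon, bat or broom.
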(event Custom|Event%20ResolveHit
  ;[1 1 1] Resolve getting hit
  (if (and (Variables|Default|GetBlocking) (!= (Variables|Default|GetSword%20Offset) (Variables|Default|GetHit%20Offset)))
    (Development|PrintString "Blocked")
    (else
      (Development|PrintString "Hit"))))

(event Input|EnhancedActionEvents|EnhancedInputActionIA_Move
  (params (ActionValue :type Vector%202D%20Structure) (ElapsedSeconds :type Float%20%28double-precision%29) (TriggeredSeconds :type Float%20%28double-precision%29) (InputAction :type Input%20Action%20Object%20Reference :default "/Game/Blueprints/Characters/Player/IA_Move.IA_Move"))
  (bind _returnvalue (Pawn|GetControlRotation :!class /Script/Engine.Pawn))
  (bind (_x _y) (Math|Vector2D|BreakVector2D ActionValue))
  (bind _returnvalue_2 (Math|Vector|GetRightVector _returnvalue))
  (bind (_x_2 _y_2 _z) (Math|Vector|BreakVector _returnvalue_2))
  ;[1 1 1] Handle directional movement
  (Pawn|Input|AddMovementInput (Math|Vector|MakeVector _y_2 (* _x_2 -1.0) _z) _x false)
  (Pawn|Input|AddMovementInput (Math|Vector|GetRightVector (Pawn|GetControlRotation :!class /Script/Engine.Pawn)) _y false))

(event Input|EnhancedActionEvents|EnhancedInputActionIA_Look
  (params (ActionValue :type Vector%202D%20Structure) (ElapsedSeconds :type Float%20%28double-precision%29) (TriggeredSeconds :type Float%20%28double-precision%29) (InputAction :type Input%20Action%20Object%20Reference :default "/Game/Blueprints/Characters/Player/IA_Look.IA_Look"))
  (bind (_x _y) (Math|Vector2D|BreakVector2D ActionValue))
  ;[1 1 1] Handle rotational movement
  (Pawn|Input|AddControllerYawInput (* (Variables|Default|GetSensitivity) _x))
  (Pawn|Input|AddControllerPitchInput (* (* _y -1.0) (Variables|Default|GetSensitivity))))

(event Input|EnhancedActionEvents|EnhancedInputActionIA_Jump
  (params (ActionValue :type Boolean) (ElapsedSeconds :type Float%20%28double-precision%29) (TriggeredSeconds :type Float%20%28double-precision%29) (InputAction :type Input%20Action%20Object%20Reference :default "/Game/Blueprints/Characters/Player/IA_Jump.IA_Jump"))
  ;[1 1 1] Handle directional movement
  (Character|Jump))

(event Input|EnhancedActionEvents|EnhancedInputActionIA_ShiftSword
  (params (ActionValue :type Float%20%28double-precision%29) (ElapsedSeconds :type Float%20%28double-precision%29) (TriggeredSeconds :type Float%20%28double-precision%29) (InputAction :type Input%20Action%20Object%20Reference :default "/Game/Blueprints/Characters/Player/IA_ShiftSword.IA_ShiftSword"))
  (bind _mesh (Variables|Character|GetMesh))
  (bind _returnvalue (Transformation|GetWorldScale _mesh))
  ;[1 1 1] Handle rotational movement
  (if (and (!= (Variables|Default|GetAttack) true) (!= (Variables|Default|GetBlocking) true))
    (if (> ActionValue 0.0)
      (Variables|Default|SetSword%20Offset 1.0)
      (if (Variables|Default|GetSwordLeftSide)
        (Variables|Default|SetSwordLeftSide false)
        (Transformation|SetWorldScale3D _mesh (Math|Vector|MakeVector (* (.x _returnvalue) -1.0) (.y _returnvalue) (.z _returnvalue)) :!label _label))
      (else
        (Variables|Default|SetSword%20Offset -1.0)
        (if (!= (Variables|Default|GetSwordLeftSide) true)
          (Variables|Default|SetSwordLeftSide true)
          (goto _label))))))

(event Input|EnhancedActionEvents|EnhancedInputActionIA_Attack
  (params (ActionValue :type Boolean) (ElapsedSeconds :type Float%20%28double-precision%29) (TriggeredSeconds :type Float%20%28double-precision%29) (InputAction :type Input%20Action%20Object%20Reference :default "/Game/Blueprints/Characters/Player/IA_Attack.IA_Attack"))
  (bind _self self)
  (bind _mesh (Variables|Character|GetMesh _self))
  ;[1 1 1] Check attack input
  (if (Math|Boolean|ANDBoolean ActionValue (!= (Variables|Default|GetBlocking) true) (!= (Variables|Default|GetAttack) true))
    (Variables|Default|SetAttack true)
    (if (> (Variables|Default|GetSword%20Offset) 0.0)
      (bind _notifyname (Animation|Montage|PlayMontage _mesh "/Game/Blueprints/Characters/Player/AM_SlashRight.AM_SlashRight")
        (:then
          (Variables|Default|SetSensitivity 0.2))
        (:OnNotifyBegin
          (switch string (Utilities|String|ToString(Name) _notifyname)
            (:AttackEnd
              (Variables|Default|SetAttack false)))))
      (else
        (bind _notifyname_2 (Animation|Montage|PlayMontage _mesh "/Game/Blueprints/Characters/Player/AM_SlashRight.AM_SlashRight")
          (:then
            (Variables|Default|SetSensitivity 0.1))
          (:OnNotifyBegin
            (switch string (Utilities|String|ToString(Name) _notifyname_2)
              (:AttackEnd
                (Variables|Default|SetAttack false)))))))))

(event Input|EnhancedActionEvents|EnhancedInputActionIA_Block
  (params (ActionValue :type Boolean) (ElapsedSeconds :type Float%20%28double-precision%29) (TriggeredSeconds :type Float%20%28double-precision%29) (InputAction :type Input%20Action%20Object%20Reference :default "/Game/Blueprints/Characters/Player/IA_Block.IA_Block"))
  (bind _self self)
  (bind _mesh (Variables|Character|GetMesh _self))
  ;[1 1 1] Handle block input
  (if (Math|Boolean|ANDBoolean ActionValue (!= (Variables|Default|GetBlocking) true) (!= (Variables|Default|GetAttack) true))
    (if (> (Variables|Default|GetSword%20Offset) 0.0)
      (Animation|Montage|PlayMontage _mesh "/Game/Blueprints/Characters/Player/AM_BlockRight.AM_BlockRight" 2.0
        (:then
          (Variables|Default|SetBlocking true)
          (Variables|Default|SetSensitivity 0.2 :!label _label))
        (:OnCompleted
          (Variables|Default|SetBlocking false)))
      (else
        (Animation|Montage|PlayMontage _mesh "/Game/Blueprints/Characters/Player/AM_BlockLeft.AM_BlockLeft" 2.0
          (:then
            (Variables|Default|SetBlocking true)
            (goto _label))
          (:OnCompleted
            (Variables|Default|SetBlocking false)))))))

(event Input|EnhancedActionEvents|EnhancedInputActionIA_OpenChest
  (params (ActionValue :type Boolean) (ElapsedSeconds :type Float%20%28double-precision%29) (TriggeredSeconds :type Float%20%28double-precision%29) (InputAction :type Input%20Action%20Object%20Reference :default "/Game/Blueprints/Characters/Player/IA_OpenChest.IA_OpenChest"))
  (bind _camera (Variables|Default|GetCamera))
  ;[1 1 1] Handle chest opening
  (bind _outactors (Actor|GetAllActorsOfClass "/Game/Blueprints/Characters/Enemy/BP_Enemy.BP_Enemy_C"))
  (bind _outhit (Collision|LineTraceForObjects (Transformation|GetWorldLocation (Variables|Collision|GetCapsuleComponent)) (+ (* (Math|Vector|GetForwardVector _camera) 2e+02) (Transformation|GetWorldLocation _camera)) (Utilities|Array|MakeArray "ObjectTypeQuery2") false _outactors "Persistent"))
  (bind _asbp_chest (Utilities|Casting|CastToBP_Chest (.hitactor _outhit)))
  (bind _randomint (Default|GetRandomInt _asbp_chest))
  (switch int _randomint
    (:0
      (Rendering|SetVisibility (Variables|Default|GetSpoon) true false)
      (Rendering|SetVisibility (Variables|Default|GetSM_BaseballBat) false false)
      (Rendering|SetVisibility (Variables|Default|GetSM_Broom) false false))
    (:1
      (Rendering|SetVisibility (Variables|Default|GetSpoon) false false)
      (Rendering|SetVisibility (Variables|Default|GetSM_BaseballBat) false false)
      (Rendering|SetVisibility (Variables|Default|GetSM_Broom) true false))
    (:2
      (Rendering|SetVisibility (Variables|Default|GetSpoon) false false)
      (Rendering|SetVisibility (Variables|Default|GetSM_BaseballBat) true false)
      (Rendering|SetVisibility (Variables|Default|GetSM_Broom) false false))))

(event EventBeginPlay
  ;[1 1 1] Set input mapping context
  (bind _asplayer_controller (Utilities|Casting|CastToPlayerController (Pawn|GetController)))
  (Input|AddMappingContext (PlayerController|LocalPlayerSubsystems|GetEnhancedInputLocalPlayerSubsystem _asplayer_controller) "/Game/Blueprints/Characters/Player/IMC_CharacterBase.IMC_CharacterBase" 0 "(bIgnoreAllPressedKeysUntilRelease=True,bForceImmediately=False,bNotifyUserSettings=False)")
  ;[1 1 1] Set sensitivity
  (Variables|Default|SetSensitivity 1.0))

(event Collision|EventActorBeginOverlap
  (params (OtherActor :type Actor%20Object%20Reference)))

(event EventTick
  (params (DeltaSeconds :type Float%20%28single-precision%29))
  (bind _returnvalue (Character|CanJump))
  ;[1 1 1] Set grounded
  (Variables|Default|SetGrounded _returnvalue)
  (bind _asabp_character_base (Utilities|Casting|CastToABP_CharacterBase (Components|SkeletalMesh|GetAnimInstance (Variables|Character|GetMesh))))
  (Variables|/Game/Blueprints/Characters/Player/ABP_CharacterBase.ABP_CharacterBase_C|SetGrounded _asabp_character_base _returnvalue)
  ;[1 1 1] Increase sensitivity to default
  (Variables|Default|SetSensitivity (Math|Float|Lerp (Variables|Default|GetSensitivity) 1.0 (* DeltaSeconds 0.5))))

(fn ConstructionScript)

(fn HitDetection
  (bind _mesh (Variables|Character|GetMesh))
  (bind _swordcollider (Variables|Default|GetSwordCollider))
  (bind _returnvalue (Transformation|GetSocketLocation _mesh "hand_r"))
  (bind _outhits (Class|KismetSystemLibrary|LineTraceMultiforObjects _returnvalue (+ _returnvalue (* (* (Components|Capsule|GetScaledCapsuleHalfHeight _swordcollider) 2.0) (Math|Vector|GetUpVector _swordcollider))) (Utilities|Array|MakeArray "ObjectTypeQuery3") false 0 "None" true))
  (for _array_element _outhits
    (bind _asbp_enemy (Utilities|Casting|CastToBP_Enemy (.HitActor (Collision|BreakHitResult _array_element))))
    (Default|EventResolveHit _asbp_enemy)))

(fn ResolveHit
  (params (Hit%20Offset :type Float%20%28double-precision%29))
  (Variables|Default|SetHit%20Offset Hit%20Offset)
  (CallFunction|EventResolveHit))