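; Base character Blueprint with Enhanced Input movement, look, jump and left/right sword slashes.
; Movement follows the control rotation's right vector, rotated for forward, and a shift input sets the sword side that picks the slash montage.
; An attack flag blocks repeats until a NotAttacking notify, with montages played on player pawn 0.
; Grounded clears on jump, updates from flat hit normals and is pushed to the anim instance.
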(event Input|EnhancedActionEvents|EnhancedInputActionIA_Move
  (params (ActionValue :type Vector%202D%20Structure) (ElapsedSeconds :type Float%20%28double-precision%29) (TriggeredSeconds :type Float%20%28double-precision%29) (InputAction :type Input%20Action%20Object%20Reference :default "/Game/Blueprints/Characters/CharacterBase/IA_Move.IA_Move"))
  (bind _returnvalue (Pawn|GetControlRotation :!class /Script/Engine.Pawn))
  (bind (_x _y) (Math|Vector2D|BreakVector2D ActionValue))
  (bind _returnvalue_2 (Math|Vector|GetRightVector _returnvalue))
  (bind (_x_2 _y_2 _z) (Math|Vector|BreakVector _returnvalue_2))
  ;[1 1 1] Handle directional movement
  (Pawn|Input|AddMovementInput (Math|Vector|MakeVector _y_2 (* _x_2 -1.0) _z) _x false)
  (Pawn|Input|AddMovementInput (Math|Vector|GetRightVector (Pawn|GetControlRotation :!class /Script/Engine.Pawn)) _y false))

(event Input|EnhancedActionEvents|EnhancedInputActionIA_Look
  (params (ActionValue :type Vector%202D%20Structure) (ElapsedSeconds :type Float%20%28double-precision%29) (TriggeredSeconds :type Float%20%28double-precision%29) (InputAction :type Input%20Action%20Object%20Reference :default "/Game/Blueprints/Characters/CharacterBase/IA_Look.IA_Look"))
  (bind (_x _y) (Math|Vector2D|BreakVector2D ActionValue))
  ;[1 1 1] Handle rotational movement
  (Pawn|Input|AddControllerYawInput _x)
  (Pawn|Input|AddControllerPitchInput (* _y -1.0)))

(event Input|EnhancedActionEvents|EnhancedInputActionIA_Jump
  (params (ActionValue :type Boolean) (ElapsedSeconds :type Float%20%28double-precision%29) (TriggeredSeconds :type Float%20%28double-precision%29) (InputAction :type Input%20Action%20Object%20Reference :default "/Game/Blueprints/Characters/CharacterBase/IA_Jump.IA_Jump"))
  ;[1 1 1] Handle directional movement
  (Character|Jump)
  (bind _output_get (Variables|Default|SetGrounded false))
  (bind _asabp_character_base (Utilities|Casting|CastToABP_CharacterBase (Components|SkeletalMesh|GetAnimInstance (Variables|Character|GetMesh))))
  (Variables|/Game/Blueprints/Characters/CharacterBase/ABP_CharacterBase.ABP_CharacterBase_C|SetGrounded _asabp_character_base _output_get))

(event Input|EnhancedActionEvents|EnhancedInputActionIA_ShiftSword
  (params (ActionValue :type Float%20%28double-precision%29) (ElapsedSeconds :type Float%20%28double-precision%29) (TriggeredSeconds :type Float%20%28double-precision%29) (InputAction :type Input%20Action%20Object%20Reference :default "/Game/Blueprints/Characters/CharacterBase/IA_ShiftSword.IA_ShiftSword"))
  ;[1 1 1] Handle rotational movement
  (if (> ActionValue 0.0)
    (Variables|Default|SetSword%20Offset 1.0)
    (else
      (Variables|Default|SetSword%20Offset -1.0))))

(event Input|EnhancedActionEvents|EnhancedInputActionIA_Attack
  (params (ActionValue :type Boolean) (ElapsedSeconds :type Float%20%28double-precision%29) (TriggeredSeconds :type Float%20%28double-precision%29) (InputAction :type Input%20Action%20Object%20Reference :default "/Game/Blueprints/Characters/CharacterBase/IA_Attack.IA_Attack"))
  ;[1 1 1] Check attack input
  (if ActionValue
    (if (!= (Variables|Default|GetAttack) true)
      (Variables|Default|SetAttack true)
      (bind _ascharacter_base (Utilities|Casting|CastToBP_CharacterBase (Game|Player|GetPlayerPawn 0)))
      (if (> (Variables|Default|GetSword%20Offset) 0.0)
        (bind _notifyname (Animation|Montage|PlayMontage (Variables|/Script/Engine.Character|GetMesh _ascharacter_base) "/Game/Blueprints/Characters/CharacterBase/AM_SlashRight.AM_SlashRight")
          (:OnNotifyBegin
            (if (== _notifyname "NotAttacking")
              (Variables|Default|SetAttack false))))
        (else
          (bind _notifyname_2 (Animation|Montage|PlayMontage (Variables|/Script/Engine.Character|GetMesh _ascharacter_base) "/Game/Blueprints/Characters/CharacterBase/AM_SlashLeft.AM_SlashLeft")
            (:OnNotifyBegin
              (if (== _notifyname_2 "NotAttacking")
                (Variables|Default|SetAttack false)))))))))

(event EventBeginPlay
  ;[1 1 1] Set input mapping context
  (bind _asplayer_controller (Utilities|Casting|CastToPlayerController (Pawn|GetController)))
  (Input|AddMappingContext (PlayerController|LocalPlayerSubsystems|GetEnhancedInputLocalPlayerSubsystem _asplayer_controller) "/Game/Blueprints/Characters/CharacterBase/IMC_CharacterBase.IMC_CharacterBase" 0 "(bIgnoreAllPressedKeysUntilRelease=True,bForceImmediately=False,bNotifyUserSettings=False)")
  ;[1 1 1] Set grounded
  (bind _output_get (Variables|Default|SetGrounded true))
  (bind _asabp_character_base (Utilities|Casting|CastToABP_CharacterBase (Components|SkeletalMesh|GetAnimInstance (Variables|Character|GetMesh))))
  (Variables|/Game/Blueprints/Characters/CharacterBase/ABP_CharacterBase.ABP_CharacterBase_C|SetGrounded _asabp_character_base _output_get))

(event Collision|EventActorBeginOverlap
  (params (OtherActor :type Actor%20Object%20Reference)))

(event EventTick
  (params (DeltaSeconds :type Float%20%28single-precision%29)))

(event Collision|EventHit
  (params (MyComp :type Primitive%20Component%20Object%20Reference) (Other :type Actor%20Object%20Reference) (OtherComp :type Primitive%20Component%20Object%20Reference) (bSelfMoved :type Boolean) (HitLocation :type Vector :default "0, 0, 0") (HitNormal :type Vector :default "0, 0, 0") (NormalImpulse :type Vector :default "0, 0, 0") (Hit :type Hit%20Result%20Structure%20%28by%20ref%29))
  ;[1 1 1] Set grounded
  (bind _output_get (Variables|Default|SetGrounded (== (.Z (Math|Vector|BreakVector (.ImpactNormal (Collision|BreakHitResult Hit)))) 1.0)))
  (bind _asabp_character_base (Utilities|Casting|CastToABP_CharacterBase (Components|SkeletalMesh|GetAnimInstance (Variables|Character|GetMesh))))
  (Variables|/Game/Blueprints/Characters/CharacterBase/ABP_CharacterBase.ABP_CharacterBase_C|SetGrounded _asabp_character_base _output_get))

(fn ConstructionScript)