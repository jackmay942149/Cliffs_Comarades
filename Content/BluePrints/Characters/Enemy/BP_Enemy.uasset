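; BP_Enemy is an enemy character that reacts to incoming hits by either blocking or registering a hit.
; The ResolveHit function stores the hit offset and triggers an event, which ignores hits while blocking, attacking or recently hit.
; Otherwise a coin flip either plays a left or right block montage, chosen from the offset's sign, or starts an invulnerability timer that Tick counts down.
; Outcomes only print debug strings, with no damage applied.
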(event Custom|Event%20Resolve%20Hit
  (bind _mesh (Variables|Character|GetMesh))
  ;[1 1 1] Resolve hit
  (if (Math|Boolean|ANDBoolean (!= (Variables|Default|GetBlocking) true) (!= (Variables|Default|GetHit) true) (!= (Variables|Default|GetAttacking) true))
    (if (Math|Random|RandomBool)
      (if (> (Variables|Default|GetHit%20Offset) 0.0)
        (Variables|Default|SetSwordOffset -1.0)
        (else
          (Variables|Default|SetSwordOffset 1.0)))
      (Variables|Default|SetBlocking true)
      (if (> (Variables|Default|GetSwordOffset) 0.0)
        (Animation|Montage|PlayMontage _mesh "/Game/Blueprints/Characters/Player/AM_BlockRight.AM_BlockRight" 2.0
          (:then
            (Development|PrintString "Blocked" :!label _label))
          (:OnCompleted
            (Variables|Default|SetBlocking false)))
        (else
          (Animation|Montage|PlayMontage _mesh "/Game/Blueprints/Characters/Player/AM_BlockLeft.AM_BlockLeft" 2.0
            (:then
              (goto _label))
            (:OnCompleted
              (Variables|Default|SetBlocking false)))))
      (else
        (Variables|Default|SetHit true)
        (Variables|Default|SetInvulnerableTimer 2.0)
        (Development|PrintString "Hit")))))

(event EventBeginPlay)

(event Collision|EventActorBeginOverlap
  (params (OtherActor :type Actor%20Object%20Reference)))

(event EventTick
  (params (DeltaSeconds :type Float%20%28single-precision%29))
  ;[1 1 1] Handle invulnerability
  (Variables|Default|SetInvulnerableTimer (- (Variables|Default|GetInvulnerableTimer) DeltaSeconds))
  (if (<= (Variables|Default|GetInvulnerableTimer) 0.0)
    (Variables|Default|SetHit false)))

(fn ConstructionScript)

(fn ResolveHit
  (params (HitOffset :type Float%20%28double-precision%29))
  (Variables|Default|SetHit%20Offset HitOffset)
  (CallFunction|EventResolveHit))