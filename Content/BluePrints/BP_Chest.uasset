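; BP_Chest is a chest Blueprint that randomly hides one of three item components: a spoon, a broom or a baseball bat.
; On BeginPlay it rolls a random integer, stores it in RandomInt and switches on it to hide the matching component, leaving the other two untouched.
; GetRandomInt exposes the stored roll, and the construction script is empty.
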(event EventBeginPlay
  (bind _output_get (Variables|Default|SetRandomInt (Math|Random|RandomInteger 3)))
  (switch int _output_get
    (:0
      (Rendering|SetVisibility (Variables|Default|GetSpoon_0) false false))
    (:1
      (Rendering|SetVisibility (Variables|Default|GetBroom_0) false false))
    (:2
      (Rendering|SetVisibility (Variables|Default|GetBaseball_Bat) false false))))

(fn ConstructionScript)

(fn GetRandomInt
  (return (Variables|Default|GetRandomInt)))