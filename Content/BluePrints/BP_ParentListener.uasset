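; BP_ParentListener is an actor that acts as a parent who catches the player for making too much noise.
; It finds and caches the BP_Player on BeginPlay.
; Each AddNoise call raises a noise counter; above the wake-up volume it plays the parent sound at its location, resets the counter, prints a caught message and deducts a point from the player's score.
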(event EventBeginPlay
  (bind _returnvalue (Actor|GetActorOfClass "/Game/BluePrints/Characters/Player/BP_Player.BP_Player_C"))
  (Variables|Default|SetPlayer _returnvalue))

(event Collision|EventActorBeginOverlap
  (params (OtherActor :type Actor%20Object%20Reference)))

(event EventTick
  (params (DeltaSeconds :type Float%20%28single-precision%29)))

(fn ConstructionScript)

(fn AddNoise
  (bind _output_get (Variables|Default|SetNoiseLevel (+ (Variables|Default|GetNoiseLevel) 1.0)))
  (if (> _output_get (Variables|Default|GetWakeUpVolume))
    (Audio|PlaySoundatLocation "/Game/Sounds/Parent.Parent" (Transformation|GetWorldLocation (Variables|Default|GetDefaultSceneRoot)) "0, 0, 0" 1.0 1.0 0.0 0 0 0 0)
    (Variables|Default|SetNoiseLevel 0.0)
    (Development|PrintString "Caught -1 Score")
    (bind _asbp_player (Utilities|Casting|CastToBP_Player (Variables|Default|GetPlayer)))
    (Default|AddScore _asbp_player -1)))